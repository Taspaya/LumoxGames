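; BP_Rayo is a short-lived player skill actor that damages Enemigo actors touching its sphere.
; It deactivates its Rayo component on BeginPlay, then activates it every Tick without reset.
; Sphere overlaps directly subtract a fixed amount from the enemy's Health and print debug messages.
; After a fixed delay, it flags EndedSimpleSkill on the player's ThirdPersonCharacter and destroys itself.
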(event `self.ReceiveBeginPlay`
  (`ActorComponent.Deactivate` (`self.Rayo`))
  (`KismetSystemLibrary.Delay` 5.0)
  (bind _asthird_person_character (cast `/Game/ThirdPersonBP/Blueprints/ThirdPersonCharacter` (`GameplayStatics.GetPlayerCharacter` 0)))
  (set `/Game/ThirdPersonBP/Blueprints/ThirdPersonCharacter.EndedSimpleSkill` true _asthird_person_character)
  (`self.K2_DestroyActor`))

(event `self.ReceiveTick`
  (params (DeltaSeconds :type "Float (single-precision)"))
  (`ActorComponent.Activate` (`self.Rayo`) false))

(event `self.Sphere.OnComponentBeginOverlap`
  (params (OverlappedComponent :type "PrimitiveComponent Object Reference") (OtherActor :type "Actor Object Reference") (OtherComp :type "PrimitiveComponent Object Reference") (OtherBodyIndex :type Integer) (bFromSweep :type Boolean) (SweepResult :type "HitResult Structure (by ref)"))
  (bind _asenemigo (cast `/Game/ThirdPersonBP/Blueprints/IA/Enemy/Enemigo` OtherActor))
  (`KismetSystemLibrary.PrintString` "Casted")
  (set `/Game/ThirdPersonBP/Blueprints/IA/Enemy/Enemigo.Health` (- (`/Game/ThirdPersonBP/Blueprints/IA/Enemy/Enemigo.Health` _asenemigo) 200) _asenemigo)
  (`KismetSystemLibrary.PrintString` (`KismetStringLibrary.Conv_IntToString` (`/Game/ThirdPersonBP/Blueprints/IA/Enemy/Enemigo.Health` _asenemigo))))

(fn `UserConstructionScript`)