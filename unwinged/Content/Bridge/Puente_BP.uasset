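; Bridge actor that falls when a Hurricane actor enters its Box trigger.
; The overlap prints a debug string, plays the Falling_Bridge 2D sound and starts a timeline.
; Each timeline update sets the actor's relative pitch from the track value, taking roll and yaw from the root component's current world rotation.
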(event `self.Box.OnComponentBeginOverlap`
  (params (OverlappedComponent :type "PrimitiveComponent Object Reference") (OtherActor :type "Actor Object Reference") (OtherComp :type "PrimitiveComponent Object Reference") (OtherBodyIndex :type Integer) (bFromSweep :type Boolean) (SweepResult :type "HitResult Structure (by ref)"))
  (cast `/Game/ThirdPersonBP/Blueprints/Hurricane` OtherActor)
  (`KismetSystemLibrary.PrintString` "etecto el hurricane")
  (`GameplayStatics.PlaySound2D` "/Game/Bridge/Falling_Bridge.Falling_Bridge")
  (bind (_direction _newtrack_1) (`Timeline|Timeline_0`)
    (:`Update`
      (`self.K2_SetActorRelativeRotation` (`KismetMathLibrary.MakeRotator` (.roll (`SceneComponent.K2_GetComponentRotation` (`self.DefaultSceneRoot`))) (.pitch (`KismetMathLibrary.MakeRotator` 0.0 _newtrack_1)) (.yaw (`SceneComponent.K2_GetComponentRotation` (`self.DefaultSceneRoot`))))))))

(fn `UserConstructionScript`)